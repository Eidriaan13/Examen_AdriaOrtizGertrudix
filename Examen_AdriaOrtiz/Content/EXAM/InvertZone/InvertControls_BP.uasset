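; InvertControls_BP is a trigger actor that temporarily sets the inverted-controls flag on the third-person character.
; Overlap by a ThirdPersonCharacter sets that character's IsInverted flag and arms the actor's own IsInvertedAA flag.
; While armed, Tick accumulates delta time and, after about five seconds, clears IsInverted on player pawn 0 and disarms itself.
; Further overlaps during the countdown do not restart the timer.
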(event `self.ReceiveTick`
  (params (DeltaSeconds :type "Float (single-precision)"))
  (if (`self.isInvertedAA`)
    (set `self.Timer` (+ (`self.Timer`) (`GameplayStatics.GetWorldDeltaSeconds`)))
    (if (> (`self.Timer`) 5.0)
      (set `self.Timer` 0.0)
      (bind _asthird_person_character (cast `/Game/ThirdPersonBP/Blueprints/ThirdPersonCharacter` (`GameplayStatics.GetPlayerPawn` 0)))
      (set `/Game/ThirdPersonBP/Blueprints/ThirdPersonCharacter.isInverted` false _asthird_person_character)
      (set `self.isInvertedAA` false))
    (else
      (set `self.Timer` 0.0))))

(event `self.ReceiveActorBeginOverlap`
  (params (OtherActor :type "Actor Object Reference"))
  (bind _asthird_person_character (cast `/Game/ThirdPersonBP/Blueprints/ThirdPersonCharacter` OtherActor))
  (set `/Game/ThirdPersonBP/Blueprints/ThirdPersonCharacter.isInverted` true _asthird_person_character)
  (set `self.isInvertedAA` true))

(fn `UserConstructionScript`)